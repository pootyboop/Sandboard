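; BP_GrapplePoint is a grapple target actor that gives feedback while it is aimed at.
; When aiming starts and no preview exists, it plays a target-hit sound and spawns a BP_GrapplePreview snapped to its PreviewCollision sphere.
; When aiming ends, it destroys that preview and clears the reference.
; The construction script sizes the collision sphere from HitboxRadius.
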(event EventStartAimedat
  (Variables|Default|Getpreview
    (:then)
    (:else
      (Audio|PlaySound2D "/Game/Audio/Sfx/World/target_hit_Cue.target_hit_Cue" 1.0 1.0 0.0 0 0)
      (bind _returnvalue (Game|SpawnActorfromClass "/Game/UI/Ingame/BP_GrapplePreview.BP_GrapplePreview_C" (Transformation|GetActorTransform) "Undefined" 0 0))
      (bind _output_get (Variables|Default|Setpreview _returnvalue))
      (Transformation|AttachComponentToComponent _output_get (Variables|Default|GetpreviewCollision) "None" "SnapToTarget" "SnapToTarget" "KeepRelative" true))))

(event EventEndAimedat
  (Actor|DestroyActor (Variables|Default|Getpreview))
  (Variables|Default|Setpreview 0))

(fn ConstructionScript
  (Components|Sphere|SetSphereRadius (Variables|Default|GetpreviewCollision) (Variables|Default|GethitboxRadius) true))