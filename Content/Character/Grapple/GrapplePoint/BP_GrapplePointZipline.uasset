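; Grapple point on a zipline that travels along the line while grappled.
; On grapple start it notifies the Zipline of its index and starts a fast looping timer that steps it along its forward vector, disconnecting the grapple outside zipline bounds.
; Grapple end clears the timer and has the Zipline set up its points again.
; A physics constraint actor is cleaned up on destroy, but its spawn function is unused here.
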(event Custom|Start%20Moving
  (bind _returnvalue (Utilities|Time|SetTimerbyEvent (delegate Custom|Move) 0.001 true))
  (Variables|Default|SetmoveTimer _returnvalue))

(event Custom|End%20Moving
  (Default|SetupGrapplePoints (Variables|Default|Getzipline) true))

(event Custom|Move
  (CallFunction|MoveAlong))

(event EventOnGrappleStart
  (|CallParentFunction)
  (CallFunction|StartMoving)
  (Default|OnGrappled (Variables|Default|Getzipline) (Variables|Default|Getindex)))

(event EventOnGrappleEnd
  (|CallParentFunction)
  (Utilities|Time|ClearandInvalidateTimerbyHandle (Variables|Default|GetmoveTimer))
  (CallFunction|EndMoving))

(event EventDestroyed
  (|CallParentFunction)
  (bind _physicsconstraint (Variables|Default|GetphysicsConstraint)
    (:then
      (Actor|DestroyActor _physicsconstraint))
    (:else)))

(fn ConstructionScript
  (|CallParentFunction))

(fn MoveAlong
  (bind _output_get (LocalVariables|SetnewLocation (+ (* (Transformation|GetActorForwardVector) (Variables|Default|GetziplineMoveSpeed)) (Transformation|GetActorLocation))))
  (if (Default|IsinZiplineBounds (Variables|Default|Getzipline) _output_get)
    (Transformation|SetActorLocation (LocalVariables|GetnewLocation) false false)
    (else
      (CallFunction|DisconnectGrapple))))

(fn SetupPhysicsConstraint
  (bind _returnvalue (Game|SpawnActorfromClass "/Game/Character/Grapple/GrapplePoint/BP_ZiplinePhysics.BP_ZiplinePhysics_C" (Transformation|GetActorTransform) "Undefined" 0 self 0))
  (bind _output_get (Variables|Default|SetphysicsConstraint _returnvalue))
  (Transformation|AttachActorToActor _output_get self "None" "SnapToTarget" "SnapToTarget" "KeepRelative" true))