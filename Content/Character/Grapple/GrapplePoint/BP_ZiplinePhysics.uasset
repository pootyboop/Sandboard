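; Physics helper actor for ziplines in the VR grapple system that tethers the player to a zipline point while the actor exists.
; On BeginPlay it enables physics simulation on the player's VR root and joins it to the zipline point's preview collision through a physics constraint.
; Destroying the actor turns the root's simulation back off.
; Tick prints the constraint's current Swing2 angle as debug output.
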(event EventBeginPlay
  (bind _returnvalue (Game|Player|GetPlayerPawn 0))
  (bind _asvive_pawn_character (Utilities|Casting|CastToPlayer _returnvalue))
  (bind _vrrootreference (Variables|/Script/VRExpansionPlugin.VRCharacter|GetVRRootReference _asvive_pawn_character))
  (Physics|SetSimulatePhysics _vrrootreference true)
  (Class|PhysicsConstraintComponent|SetConstrainedComponents (Variables|Default|GetPhysicsConstraint) _vrrootreference "None" (Variables|/Game/Character/Grapple/GrapplePoint/BP_GrapplePoint.BP_GrapplePoint_C|GetpreviewCollision (Variables|Default|GetziplinePoint)) "None"))

(event EventTick
  (params (DeltaSeconds :type Float%20%28single-precision%29))
  (Development|PrintString (Utilities|String|ToString(Float) (Class|PhysicsConstraintComponent|GetCurrentSwing2 (Variables|Default|GetPhysicsConstraint)))))

(event EventDestroyed
  (Physics|SetSimulatePhysics (Variables|/Script/VRExpansionPlugin.VRCharacter|GetVRRootReference (.AsVive%20Pawn%20Character (Utilities|Casting|CastToPlayer (Game|Player|GetPlayerPawn 0)))) false))

(fn ConstructionScript)