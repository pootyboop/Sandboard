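; BP_GrappleHook is a grapple hook projectile that can home in on a target grapple point.
; On BeginPlay it applies its mesh and launch velocity, then SetupHoming switches to homing from zero velocity if a target point is valid.
; IgnoreHook excludes another hook from movement collision.
; An unused OldCollisionSetup ignores the Vive pawn and its pistols, and pairs mutual ignores with the other hook.
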(event Custom|Ignore%20Hook
  (params (Hook :type BP%20Grapple%20Hook%20Object%20Reference))
  (Utilities|IsValid Hook
    (:Is%20Valid
      (Collision|IgnoreActorwhenMoving (Variables|Default|GetStaticMesh) Hook true))))

(event EventBeginPlay
  (Components|StaticMesh|SetStaticMesh (Variables|Default|GetStaticMesh) (Variables|Default|Getmesh))
  (Variables|/Script/Engine.MovementComponent|SetVelocity (Variables|Default|GetProjectileMovement) (Variables|Default|GetVelocity))
  (CallFunction|SetupHoming))

(fn ConstructionScript)

(fn OldCollisionSetup
  (bind _returnvalue (Game|Player|GetPlayerPawn 0))
  (bind _otherhook (Variables|Default|GetotherHook))
  (bind _asvive_pawn_character (Utilities|Casting|CastToVive_PawnCharacter _returnvalue))
  (Utilities|FlowControl|Sequence
    (:then_0
      (Collision|IgnoreActorwhenMoving (Variables|Default|GetStaticMesh) _returnvalue true)
      (Collision|IgnoreActorwhenMoving (Variables|Default|GetStaticMesh) (Variables|/Game/Character/Vive_PawnCharacter.Vive_PawnCharacter_C|GetPistolL _asvive_pawn_character) true)
      (Collision|IgnoreActorwhenMoving (Variables|Default|GetStaticMesh) (Variables|/Game/Character/Vive_PawnCharacter.Vive_PawnCharacter_C|GetPistolR _asvive_pawn_character) true))
    (:then_1
      (Utilities|IsValid _otherhook
        (:Is%20Valid
          (CallFunction|IgnoreHook _otherhook)
          (CallFunction|IgnoreHook _otherhook self))))))

(fn SetupHoming
  (Variables|Default|GettargetGrapplePoint
    (:then
      (Variables|/Script/Engine.ProjectileMovementComponent|SetbIsHomingProjectile (Variables|Default|GetProjectileMovement) true)
      (Variables|/Script/Engine.ProjectileMovementComponent|SetHomingTargetComponent (Variables|Default|GetProjectileMovement) (Variables|/Script/Engine.Actor|GetRootComponent (Variables|Default|GettargetGrapplePoint)))
      (Variables|/Script/Engine.MovementComponent|SetVelocity (Variables|Default|GetProjectileMovement) "0, 0, 0"))
    (:else)))