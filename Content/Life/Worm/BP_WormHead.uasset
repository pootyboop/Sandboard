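; BP_WormHead is the head of a worm creature and gives it a periodic roar sound.
; It first roars a few seconds after BeginPlay, spawning the roar cue attached to its skeletal mesh.
; Each roar schedules the next with a one-shot timer at a random interval, forming an endless, irregular loop.
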(event Custom|roarTimer
  (Utilities|Time|SetTimerbyEvent (delegate Custom|Roar) (Math|Random|RandomFloatinRange 1e+01 18.0)))

(event Custom|Roar
  (Audio|SpawnSoundAttached "/Game/Audio/Sfx/Life/worm_roar_Cue.worm_roar_Cue" (Variables|Default|GetSkeletalMesh) "None" "0, 0, 0" "0, 0, 0" "SnapToTarget" false 1.0 1.0 0.0 0 0)
  (CallFunction|RoarTimer))

(event EventBeginPlay
  (|CallParentFunction)
  (Utilities|FlowControl|Delay 5.5)
  (CallFunction|Roar))

(fn ConstructionScript
  (|CallParentFunction))