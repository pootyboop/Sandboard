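; BP_Worm is a spawner actor that builds a segmented worm along a referenced spline on BeginPlay.
; It spawns a BP_WormHead at index 0 and BP_WormSegment actors behind it, flagging the second-to-last loop index as the tail.
; Each gets a start offset staggered by index and adjusted for spline length and segment spacing.
; Width and height taper toward the rear, except when IsBoost keeps the scale uniform.
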(event EventBeginPlay
  (CallFunction|BuildWorm))

(fn ConstructionScript)

(fn BuildWorm
  (bind _returnvalue (Transformation|GetActorTransform))
  (for _index (range 0 (Variables|Default|GetnumOfSegments))
    (bind _newsegment (CallFunction|SpawnSegment (select (Variables|Default|GetisBoost) (Transformation|GetActorTransform) (Math|Transform|MakeTransform (.location _returnvalue) (.rotation _returnvalue) (Math|Vector|MakeVector (* (.x (.scale _returnvalue)) (Math|Float|Lerp 1.0 0.3 (/ (Math|Conversions|ToFloat(Integer) _index) (Math|Conversions|ToFloat(Integer) (Variables|Default|GetnumOfSegments))))) (.y (.scale _returnvalue)) (* (.z (.scale _returnvalue)) (Math|Float|Lerp 1.0 0.3 (/ (Math|Conversions|ToFloat(Integer) _index) (Math|Conversions|ToFloat(Integer) (Variables|Default|GetnumOfSegments)))))))) _index (/ (* (- (Variables|Default|GetnumOfSegments) _index) 0.003) (/ (Spline|GetSplineLength (Variables|/Game/Life/_SplineMovement/BP_SplinePath.BP_SplinePath_C|GetSpline (Variables|Default|Getspline))) (Variables|Default|GetdistanceBetweenSegments)))))
    (Utilities|Array|Add (Variables|Default|Getsegments) _newsegment)
    (Default|SetPositionAlongSpline _newsegment 0.0)))

(fn SpawnSegment
  (params (SpawnTransform :type Transform) (index :type Integer) (startingPosition :type Float%20%28single-precision%29))
  (if (== index 0)
    (bind _returnvalue (Game|SpawnActorfromClass "/Game/Life/Worm/BP_WormHead.BP_WormHead_C" SpawnTransform "Undefined" 0 index (Variables|Default|Getspline) startingPosition false false 0))
    (return _returnvalue)
    (else
      (bind _returnvalue_2 (Game|SpawnActorfromClass "/Game/Life/Worm/BP_WormSegment.BP_WormSegment_C" SpawnTransform "Undefined" 0 index (Variables|Default|Getspline) startingPosition (Variables|Default|GetisBoost) (== index (- (Variables|Default|GetnumOfSegments) 1)) 0))
      (return _returnvalue_2))))