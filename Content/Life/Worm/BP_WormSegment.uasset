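; BP_WormSegment is one body segment of a sandworm that travels repeatedly along a spline, spinning its mesh as it moves.
; A looping timeline, rate-scaled by spline length for constant speed, drives position and rotation.
; The construction script offsets mesh rotation by segment index, swaps in a tail mesh when flagged, and strips the Boost component from non-boost segments.
; Sphere overlaps entering or leaving "wormsand"-tagged actors spawn sand Niagara effects.
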(event OnComponentBeginOverlap(Sphere)
  (params (OverlappedComponent :type Primitive%20Component%20Object%20Reference) (OtherActor :type Actor%20Object%20Reference) (OtherComp :type Primitive%20Component%20Object%20Reference) (OtherBodyIndex :type Integer) (bFromSweep :type Boolean) (SweepResult :type Hit%20Result%20Structure%20%28by%20ref%29))
  (CallFunction|OverlapSand OtherActor))

(event OnComponentEndOverlap(Sphere)
  (params (OverlappedComponent :type Primitive%20Component%20Object%20Reference) (OtherActor :type Actor%20Object%20Reference) (OtherComp :type Primitive%20Component%20Object%20Reference) (OtherBodyIndex :type Integer))
  (CallFunction|OverlapSand OtherActor))

(event Custom|StartTimeline
  (Components|Timeline|SetPlayRate (Variables|Default|GetmoveTL) (/ 1.0 (Variables|Default|GettimeToComplete)))
  (Utilities|FlowControl|Sequence
    (:then_0
      (bind _movement (Timeline|moveTL SetNewTime)
        (:Update
          (CallFunction|SetPositionAlongSpline _movement))
        (:Finished
          (CallFunction|RestartTimeline))))
    (:then_1
      (Timeline|moveTL Play))))

(event Custom|RestartTimeline
  (CallFunction|SetPositionAlongSpline 0.0)
  (bind _movement (Timeline|moveTL PlayFromStart)
    (:Update
      (CallFunction|SetPositionAlongSpline _movement))
    (:Finished
      (CallFunction|RestartTimeline))))

(event EventBeginPlay
  (CallFunction|StartTimeline))

(fn ConstructionScript
  (CallFunction|UpdateTail)
  (CallFunction|RotateMesh (Math|Conversions|ToFloat(Integer) (* (Variables|Default|Getindex) 10)))
  (Variables|Default|SettimeToComplete (/ (Spline|GetSplineLength (Variables|/Game/Life/Surfer/BP_SurferSplinePath.BP_SurferSplinePath_C|GetSpline (Variables|Default|Getspline))) 3e+04))
  (if (not (Variables|Default|GetisBoost))
    (Components|DestroyComponent (Variables|Default|Getboost))))

(fn SetPositionAlongSpline
  (params (Alpha :type Float%20%28single-precision%29))
  (bind _spline (Variables|Default|Getspline))
  (bind _spline_2 (Variables|/Game/Life/_SplineMovement/BP_SplinePath.BP_SplinePath_C|GetSpline _spline))
  (bind _output_get (LocalVariables|Setpos (Math|Float|Lerp 0.0 (Spline|GetSplineLength (Variables|/Game/Life/_SplineMovement/BP_SplinePath.BP_SplinePath_C|GetSpline (Variables|Default|Getspline))) Alpha)))
  (Transformation|SetActorTransform (Math|Transform|MakeTransform (Spline|GetLocationatDistanceAlongSpline _spline_2 _output_get "World") (Math|Rotator|MakeRotator (.roll (Spline|GetRotationatDistanceAlongSpline _spline_2 _output_get "World")) (.pitch (Spline|GetRotationatDistanceAlongSpline _spline_2 _output_get "World")) (.yaw (Spline|GetRotationatDistanceAlongSpline _spline_2 _output_get "World"))) (Transformation|GetActorScale3D)))
  (CallFunction|RotateMesh 1.0))

(fn RotateMesh
  (params (amount :type Float%20%28single-precision%29))
  (Transformation|AddLocalRotation (Variables|Default|GetSkeletalMesh) (Math|Rotator|MakeRotator 0.0 amount 0.0) false false))

(fn OverlapSand
  (params (overlappedActor :type Actor%20Object%20Reference))
  (bind _skeletalmesh (Variables|Default|GetSkeletalMesh))
  (bind _returnvalue (Transformation|GetWorldTransform _skeletalmesh))
  (if (Actor|ActorHasTag overlappedActor "wormsand")
    (bind _returnvalue_2 (Niagara|SpawnSystematLocation "/Game/FX/N_WormSand.N_WormSand" (.location _returnvalue) (.rotation _returnvalue) (.scale _returnvalue) true false))
    (Class|NiagaraComponent|SetForceSolo _returnvalue_2 true)
    (Components|Activation|SetActive _returnvalue_2 true false)))

(fn UpdateTail
  (if (Variables|Default|Gettail)
    (Class|SkinnedMeshComponent|SetSkeletalMesh (Variables|Default|GetSkeletalMesh) "/Game/Life/Worm/Meshes/sandworm_tail.sandworm_tail" true)))