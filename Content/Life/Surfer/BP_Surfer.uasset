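; BP_Surfer is an ambient surfer that loops along the first BP_SurferSplinePath it finds, with a randomized clothes color set at construction.
; A timeline drives its distance along the spline, with play rate derived from spline length plus random variation.
; It follows spline XY and rotation flipped 180° in yaw, taking spline height only at the start point.
; Smoke activates at BeginPlay, while Sand toggles with Particlecheck overlaps.
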(event OnComponentBeginOverlap(particlecheck)
  (params (OverlappedComponent :type Primitive%20Component%20Object%20Reference) (OtherActor :type Actor%20Object%20Reference) (OtherComp :type Primitive%20Component%20Object%20Reference) (OtherBodyIndex :type Integer) (bFromSweep :type Boolean) (SweepResult :type Hit%20Result%20Structure%20%28by%20ref%29))
  (Components|Activation|SetActive (Variables|Default|Getsand) true false))

(event OnComponentEndOverlap(particlecheck)
  (params (OverlappedComponent :type Primitive%20Component%20Object%20Reference) (OtherActor :type Actor%20Object%20Reference) (OtherComp :type Primitive%20Component%20Object%20Reference) (OtherBodyIndex :type Integer))
  (Components|Activation|SetActive (Variables|Default|Getsand) false false))

(event Custom|StartTimeline
  (Components|Timeline|SetPlayRate (Variables|Default|GetmoveTL) (/ 1.0 (Variables|Default|GettimeToComplete)))
  (Utilities|FlowControl|Sequence
    (:then_0
      (bind _movement (Timeline|moveTL SetNewTime)
        (:Update
          (CallFunction|SetPositionAlongSpline _movement))
        (:Finished
          (CallFunction|RestartTimeline))))
    (:then_1
      (Timeline|moveTL Play))))

(event Custom|RestartTimeline
  (CallFunction|SetPositionAlongSpline 0.0)
  (bind _movement (Timeline|moveTL PlayFromStart)
    (:Update
      (CallFunction|SetPositionAlongSpline _movement))
    (:Finished
      (CallFunction|RestartTimeline))))

(event EventBeginPlay
  (Setup|StartFollowingPath)
  (Components|Activation|SetActive (Variables|Default|Getsmoke) true false))

(fn ConstructionScript
  (Setup|RandomizeClothesColor))

(fn SetPositionAlongSpline
  (params (alpha :type Float%20%28single-precision%29))
  (bind _spline (Variables|Default|Getspline))
  (bind _spline_2 (Variables|/Game/Life/_SplineMovement/BP_SplinePath.BP_SplinePath_C|GetSpline _spline))
  (bind _output_get (LocalVariables|Setpos (Math|Float|Lerp 0.0 (Spline|GetSplineLength (Variables|/Game/Life/_SplineMovement/BP_SplinePath.BP_SplinePath_C|GetSpline (Variables|Default|Getspline))) alpha)))
  (Transformation|SetActorTransform (Math|Transform|MakeTransform (Math|Vector|MakeVector (.X (Math|Vector|BreakVector (Spline|GetLocationatDistanceAlongSpline _spline_2 _output_get "World"))) (.Y (Math|Vector|BreakVector (Spline|GetLocationatDistanceAlongSpline _spline_2 _output_get "World"))) (Math|Float|SelectFloat (+ (.Z (Math|Vector|BreakVector (Spline|GetLocationatDistanceAlongSpline _spline_2 _output_get "World"))) 1e+01) (.z (Transformation|GetActorLocation)) (== _output_get 0.0))) (Math|Rotator|MakeRotator (.Roll (Math|Rotator|BreakRotator (Spline|GetRotationatDistanceAlongSpline _spline_2 _output_get "World"))) (.Pitch (Math|Rotator|BreakRotator (Spline|GetRotationatDistanceAlongSpline _spline_2 _output_get "World"))) (+ (.Yaw (Math|Rotator|BreakRotator (Spline|GetRotationatDistanceAlongSpline _spline_2 _output_get "World"))) 1.8e+02)) "1,1,1")))

(fn StartFollowingPath
  (Utilities|FlowControl|Sequence
    (:then_0
      (bind _returnvalue (Actor|GetActorOfClass "/Game/Life/Surfer/BP_SurferSplinePath.BP_SurferSplinePath_C"))
      (Variables|Default|Setspline _returnvalue)
      (Setup|SetupTimetoComplete)
      (CallFunction|SetPositionAlongSpline 0.0))
    (:then_1
      (CallFunction|StartTimeline))))

(fn GetRandomClothesColor
  (bind _returnvalue (Math|Random|RandomFloat))
  (bind _returnvalue_2 (Math|Random|RandomFloat))
  (bind _returnvalue_3 (Math|Color|Lerp(LinearColor) "(R=0.393115,G=0.235557,B=0.000000,A=1.000000)" "(R=0.029243,G=0.055807,B=0.401042,A=1.000000)" _returnvalue))
  (bind _returnvalue_4 (Math|Color|Lerp(LinearColor) "(R=0.393115,G=0.066572,B=0.048532,A=1.000000)" "(R=0.023085,G=0.095000,B=0.060241,A=1.000000)" _returnvalue_2))
  (return (Math|Color|SelectColor (Math|Color|SelectColor _returnvalue_3 (Math|Color|Lerp(LinearColor) _returnvalue_4 _returnvalue_3 (Math|Random|RandomFloat)) (Math|Random|RandomBool)) _returnvalue_4 (> (Math|Random|RandomFloat) 0.7))))

(fn RandomizeClothesColor
  (bind _returnvalue (Rendering|Material|CreateDynamicMaterialInstance "/Game/Materials/zMisc/M_SurferClothes_Inst.M_SurferClothes_Inst" "None" "None" :!class /Script/Engine.KismetMaterialLibrary))
  (bind _output_get (Variables|Default|SetclothesMaterial _returnvalue))
  (Rendering|Material|SetVectorParameterValue _output_get "Color" (Setup|GetRandomClothesColor) :!class /Script/Engine.MaterialInstanceDynamic)
  (Rendering|Material|SetMaterial (Variables|Default|Getsurfer) 0 (Variables|Default|GetclothesMaterial)))

(fn SetupTimetoComplete
  (bind _spline (Variables|Default|Getspline))
  (bind _spline_2 (Variables|/Game/Life/Surfer/BP_SurferSplinePath.BP_SurferSplinePath_C|GetSpline _spline))
  (bind _returnvalue (Spline|GetSplineLength _spline_2))
  (bind _returnvalue_2 (/ _returnvalue 7e+03))
  (bind _returnvalue_3 (/ _returnvalue_2 4.0))
  (Variables|Default|SettimeToComplete (+ _returnvalue_2 (Math|Random|RandomFloatinRange (* -1 _returnvalue_3) _returnvalue_3))))