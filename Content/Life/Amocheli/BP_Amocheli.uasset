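; BP_Amocheli is a creature actor with a grapple point, moved along a path by a SplineFollowComponent.
; The construction script snaps the grapple point to a skeletal mesh socket and passes the starting position to the spline follower.
; It also gives each instance a dynamic skin material with a swirl color randomly blended between red and blue.
; Tick does nothing, and the old forward-teleport movement function is left disconnected.
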(event EventTick
  (params (DeltaSeconds :type Float%20%28single-precision%29)))

(fn ConstructionScript
  (Transformation|AttachComponentToComponent (Variables|Default|GetgrapplePoint) (Variables|Default|GetSkeletalMesh) "grapplePoint" "SnapToTarget" "KeepRelative" "KeepRelative" true)
  (CallFunction|RandomizeSwirlColor)
  (Variables|/Game/Life/_SplineMovement/SplineFollowComponent.SplineFollowComponent_C|SetstartingPosition%25 (Variables|Default|GetSplineFollowComponent) (Variables|Default|GetstartingPosition%25)))

(fn OldMovement
  (Transformation|SetActorLocation (+ (* (Math|Vector|Normalize (Math|Vector|GetForwardVector (Variables|Default|GetmoveDir))) (* (Utilities|Time|GetWorldDeltaSeconds) (Variables|Default|GetspeedOLD))) (Transformation|GetActorLocation)) false true))

(fn RandomizeSwirlColor
  (bind _returnvalue (Rendering|Material|CreateDynamicMaterialInstance "/Game/Materials/Amocheli/M_Amocheli_Skin_Inst.M_Amocheli_Skin_Inst" "None" "None" :!class /Script/Engine.KismetMaterialLibrary))
  (bind _output_get (Variables|Default|SetskinMaterial _returnvalue))
  (Rendering|Material|SetVectorParameterValue _output_get "Swirl Color" (Math|Color|Lerp(LinearColor) "(R=1.000000,G=0.030793,B=0.000000,A=1.000000)" "(R=0.114653,G=0.000000,B=1.000000,A=1.000000)" (Math|Random|RandomFloat)) :!class /Script/Engine.MaterialInstanceDynamic)
  (Rendering|Material|SetMaterial (Variables|Default|GetSkeletalMesh) 0 (Variables|Default|GetskinMaterial)))