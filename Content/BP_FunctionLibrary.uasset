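; Blueprint function library with two helpers, one for formatting a time value and one for detecting the menu level.
; ToSeconds, despite its name, peels minutes off a seconds value by repeated subtraction and returns colon-separated text with zero-padded seconds.
; It joins the parts with dots, then replaces every dot with a colon, including any decimal point in the seconds.
; InMenu compares the current level name to "Menu".
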(fn ToSeconds
  (params (Time :type Float%20%28single-precision%29))
  (LocalVariables|SettimeLeft Time)
  (while (>= (LocalVariables|GettimeLeft) 6e+01)
    (LocalVariables|SettimeLeft (- (LocalVariables|GettimeLeft) 6e+01))
    (Math|Integer|IncrementInt (LocalVariables|GetMinutes)))
  (return (Utilities|Text|ToText(String) (Utilities|String|Replace (Utilities|String|Append (Utilities|String|ToString(Integer) (LocalVariables|GetMinutes)) "." (Utilities|String|SelectString "0" "" (< (LocalVariables|GettimeLeft) 1e+01)) (Utilities|String|ToString(Text) (Utilities|Text|ToText(Float) (LocalVariables|GettimeLeft) "HalfToEven"))) "." ":"))))

(fn InMenu
  (bind _returnvalue (Game|GetCurrentLevelName 0))
  (return (Utilities|Enum|Equal(Enum) _returnvalue "Menu")))