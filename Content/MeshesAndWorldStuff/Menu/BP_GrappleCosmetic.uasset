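; Menu world pickup that lets the player change the cosmetic mesh of their grapple hook.
; On Interact or any sphere overlap, it swaps its GrappleMesh with the pawn's left hook mesh, refreshes its two display meshes and saves the game.
; Two seconds after BeginPlay, it switches to the Grapple mesh if its own mesh matches the equipped one, avoiding a duplicate.
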(event OnComponentBeginOverlap(Sphere)
  (params (OverlappedComponent :type Primitive%20Component%20Object%20Reference) (OtherActor :type Actor%20Object%20Reference) (OtherComp :type Primitive%20Component%20Object%20Reference) (OtherBodyIndex :type Integer) (bFromSweep :type Boolean) (SweepResult :type Hit%20Result%20Structure%20%28by%20ref%29))
  (CallFunction|SetGrapple))

(event EventInteract
  (CallFunction|SetGrapple))

(event EventBeginPlay
  (Utilities|FlowControl|Delay 2.0)
  (if (== (Variables|Default|GetgrappleMesh) (Variables|/Script/Engine.StaticMeshComponent|GetStaticMesh (Variables|/Game/Character/Vive_PawnCharacter.Vive_PawnCharacter_C|GetHookLeft (.AsVive%20Pawn%20Character (Utilities|Casting|CastToVive_PawnCharacter (Game|Player|GetPlayerPawn 0))))))
    (Variables|Default|SetgrappleMesh "/Game/Character/Grapple/Grapple.Grapple")
    (CallFunction|UpdateMesh)))

(fn ConstructionScript
  (CallFunction|UpdateMesh))

(fn SetGrapple
  (bind _returnvalue (Game|Player|GetPlayerPawn 0))
  (bind _asvive_pawn_character (Utilities|Casting|CastToVive_PawnCharacter _returnvalue))
  (LocalVariables|Settemp (Variables|/Script/Engine.StaticMeshComponent|GetStaticMesh (Variables|/Game/Character/Vive_PawnCharacter.Vive_PawnCharacter_C|GetHookLeft _asvive_pawn_character)))
  (Default|SetGrappleMesh _asvive_pawn_character (Variables|Default|GetgrappleMesh))
  (Variables|Default|SetgrappleMesh (LocalVariables|Gettemp))
  (CallFunction|UpdateMesh)
  (CallFunction|SaveGame "save"))

(fn UpdateMesh
  (Components|StaticMesh|SetStaticMesh (Variables|Default|GetMesh) (Variables|Default|GetgrappleMesh))
  (Components|StaticMesh|SetStaticMesh (Variables|Default|GetMesh1) (Variables|Default|GetgrappleMesh)))