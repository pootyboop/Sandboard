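; BP_SettingsTable is the menu's settings table, pairing a W_Settings widget with a set of table props for each settings page (customization, playstyle).
; SetScreen steps left or right through the ESettingsPage enum with wraparound, starts the widget's page transition and refreshes its text after a short timer delay.
; UpdateTableStuff swaps props by teleporting the previous page's component far below and the current one to its origin.
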(event Custom|WidgetAnimationDelay
  (Utilities|Time|SetTimerbyEvent (delegate Custom|UpdateWidgetText) 0.15))

(event Custom|UpdateWidgetText
  (Default|UpdateText (Variables|Default|GetwidgetRef)))

(event EventBeginPlay
  (bind _output_get (Variables|Default|SetwidgetRef (.AsW%20Settings (Utilities|Casting|CastToW_Settings (UserInterface|GetUserWidgetObject (Variables|Default|GetUI))))))
  (Variables|/Game/UI/Menu/Settings/W_Settings.W_Settings_C|Settable _output_get self)
  (CallFunction|UpdateTableStuff))

(fn ConstructionScript)

(fn SetScreen
  (params (previousScreen :type ESettingsPage%20Enum :default "NewEnumerator0") (isRight :type Boolean))
  (Variables|Default|SetlastScreen previousScreen)
  (Utilities|FlowControl|Sequence
    (:then_0
      (LocalVariables|SetfinalPageIndex (Math|Conversions|ToByte(Integer) (- (|GetNumEnumEntries) 1)))
      (if (and (== previousScreen 0) (not isRight))
        (Variables|Default|SetcurrentScreen (Utilities|Enum|ByteToEnumESettingsPage (LocalVariables|GetfinalPageIndex)))
        (elif (and (== previousScreen (LocalVariables|GetfinalPageIndex)) isRight)
          (Variables|Default|SetcurrentScreen (Utilities|Enum|ByteToEnumESettingsPage))
          (else
            (Variables|Default|SetcurrentScreen (Utilities|Enum|ByteToEnumESettingsPage (select isRight (+ previousScreen 1) (- previousScreen 1))))))))
    (:then_1
      (Default|StartNewPageTransition (Variables|Default|GetwidgetRef) (Utilities|Text|ToText(String) (Utilities|String|EnumtoString (Variables|Default|GetcurrentScreen))) isRight)
      (CallFunction|WidgetAnimationDelay)
      (CallFunction|UpdateTableStuff))))

(fn UpdateTableStuff
  (Transformation|SetRelativeLocation (CallFunction|GetTableStuff (Variables|Default|GetlastScreen)) "0, 0,-10000.000000" false true)
  (Transformation|SetRelativeLocation (CallFunction|GetTableStuff (Variables|Default|GetcurrentScreen)) "0, 0, 0" false true))

(fn GetTableStuff
  (params (screen :type ESettingsPage%20Enum :default "NewEnumerator0"))
  (return (Utilities|Select :Index screen :NewEnumerator0 (Variables|Default|GetCUSTOMIZATION) :NewEnumerator1 (Variables|Default|GetPLAYSTYLE))))