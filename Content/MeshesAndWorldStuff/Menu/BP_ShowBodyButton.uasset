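; VR menu button that toggles whether the player's IK body is shown.
; On BeginPlay it reads the saved ShowBody setting and updates its label to a green VISIBLE or red HIDDEN.
; Each press plays a sound, flips the state, applies it to the player pawn, saves to the "save" slot and refreshes the label.
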(event OnButtonBeginInteraction(VRButton)
  (params (InteractingActor :type Actor%20Object%20Reference) (InteractingComponent :type Primitive%20Component%20Object%20Reference))
  (Audio|PlaySound2D "/Game/Audio/Sfx/UI/ShowBody.ShowBody" 1.0 1.0 0.0 0 0)
  (CallFunction|SetBodyVisibility (not (Variables|Default|GetbodyVisible))))

(event EventBeginPlay
  (|CallParentFunction)
  (Variables|Default|SetbodyVisible (Variables|/Game/_Global/BP_SaveGame.BP_SaveGame_C|GetshowBody (CallFunction|LoadSaveGame "save")))
  (CallFunction|UpdateButtonAppearance))

(fn ConstructionScript
  (|CallParentFunction))

(fn SetBodyVisibility
  (params (visibility :type Boolean))
  (bind _output_get (Variables|Default|SetbodyVisible visibility))
  (Default|SetIKBodyVisibility (.AsPlayer (Utilities|Casting|CastToPlayer (Game|Player|GetPlayerPawn 0))) _output_get)
  (CallFunction|SaveGame "save")
  (CallFunction|UpdateButtonAppearance))

(fn UpdateButtonAppearance
  (Default|UpdateText (Variables|Default|GetwidgetRef) (select (Variables|Default|GetbodyVisible) "VISIBLE" "HIDDEN") (select (Variables|Default|GetbodyVisible) (Utilities|Struct|MakeSlateColor "(R=0.000000,G=1.000000,B=0.000000,A=1.000000)") (Utilities|Struct|MakeSlateColor "(R=1.000000,G=0.000000,B=0.000000,A=1.000000)"))))