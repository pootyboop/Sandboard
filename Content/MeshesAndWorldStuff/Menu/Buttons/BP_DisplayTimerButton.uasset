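; BP_DisplayTimerButton is a VR menu button that toggles whether the timer display setting is on or off.
; On BeginPlay it reads DisplayTimer from the "save" slot and refreshes its label.
; Pressing it plays a sound, flips the flag, writes it back to the save game, and updates the widget to green VISIBLE or dark grey HIDDEN.
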(event OnButtonBeginInteraction(VRButton)
  (params (InteractingActor :type Actor%20Object%20Reference) (InteractingComponent :type Primitive%20Component%20Object%20Reference))
  (Audio|PlaySound2D "/Game/Audio/Sfx/World/level_complete_Cue.level_complete_Cue" 1.0 1.0 0.0 0 0)
  (CallFunction|SetDisplayTimer (not (Variables|Default|GetdisplayTimer))))

(event EventBeginPlay
  (|CallParentFunction)
  (Variables|Default|SetdisplayTimer (Variables|/Game/_Global/BP_SaveGame.BP_SaveGame_C|GetdisplayTimer (CallFunction|LoadSaveGame "save")))
  (CallFunction|UpdateButtonAppearance))

(fn ConstructionScript
  (|CallParentFunction))

(fn SetDisplayTimer
  (params (display :type Boolean))
  (bind _output_get (Variables|Default|SetdisplayTimer display))
  (bind _output_get_2 (LocalVariables|SetsaveRef (CallFunction|LoadSaveGame "save")))
  (Variables|/Game/_Global/BP_SaveGame.BP_SaveGame_C|SetdisplayTimer _output_get_2 _output_get)
  (SaveGame|SaveGametoSlot (LocalVariables|GetsaveRef) "save")
  (CallFunction|UpdateButtonAppearance))

(fn UpdateButtonAppearance
  (Default|UpdateText (Variables|Default|GetwidgetRef) (select (Variables|Default|GetdisplayTimer) "VISIBLE" "HIDDEN") (select (Variables|Default|GetdisplayTimer) (Utilities|Struct|MakeSlateColor "(R=0.000000,G=1.000000,B=0.000000,A=1.000000)") (Utilities|Struct|MakeSlateColor "(R=0.078125,G=0.078125,B=0.078125,A=1.000000)"))))