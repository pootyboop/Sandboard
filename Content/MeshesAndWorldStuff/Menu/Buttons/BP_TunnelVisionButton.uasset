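; VR menu button that toggles the player's tunnel vision setting.
; On begin play it reads the flag from the "save" slot; each press flips it, plays a select sound, applies it to the player pawn and writes it back to the save.
; An appearance update sets an ENABLED/DISABLED label in green or dark gray and swaps the on/off visor components to match.
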(event OnButtonBeginInteraction(VRButton)
  (params (InteractingActor :type Actor%20Object%20Reference) (InteractingComponent :type Primitive%20Component%20Object%20Reference))
  (Audio|PlaySound2D "/Game/Audio/Sfx/Player/select.select" 1.0 1.0 0.0 0 0)
  (CallFunction|SetTunnelVision (not (Variables|Default|GettunnelVision))))

(event EventBeginPlay
  (|CallParentFunction)
  (Variables|Default|SettunnelVision (Variables|/Game/_Global/BP_SaveGame.BP_SaveGame_C|GettunnelVision (CallFunction|LoadSaveGame "save")))
  (CallFunction|UpdateButtonAppearance))

(fn ConstructionScript
  (|CallParentFunction))

(fn SetTunnelVision
  (params (tunnelVision :type Boolean))
  (bind _output_get (Variables|Default|SettunnelVision tunnelVision))
  (Default|SetTunnelVision (.AsPlayer (Utilities|Casting|CastToPlayer (Game|Player|GetPlayerPawn 0))) _output_get)
  (bind _output_get_2 (LocalVariables|SetsaveRef (CallFunction|LoadSaveGame "save")))
  (Variables|/Game/_Global/BP_SaveGame.BP_SaveGame_C|SettunnelVision _output_get_2 tunnelVision)
  (SaveGame|SaveGametoSlot (LocalVariables|GetsaveRef) "save")
  (CallFunction|UpdateButtonAppearance))

(fn UpdateButtonAppearance
  (Default|UpdateText (Variables|Default|GetwidgetRef) (select (Variables|Default|GettunnelVision) "ENABLED" "DISABLED") (select (Variables|Default|GettunnelVision) (Utilities|Struct|MakeSlateColor "(R=0.000000,G=1.000000,B=0.000000,A=1.000000)") (Utilities|Struct|MakeSlateColor "(R=0.078125,G=0.078125,B=0.078125,A=1.000000)")))
  (Rendering|SetVisibility (Variables|Default|GetTunnelVisors) (Variables|Default|GettunnelVision) false)
  (Rendering|SetVisibility (Variables|Default|GetTunnelVisors%20Off) (not (Variables|Default|GettunnelVision)) false))