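; A menu VR button that toggles the player's target help setting on and off.
; On begin play it reads the flag from the "save" slot to set its look.
; Each press plays a sound, flips the flag, pushes it to the player pawn and writes it back to the save.
; The widget text and color, plus the visibility of the on and off components, follow the current state.
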(event OnButtonBeginInteraction(VRButton)
  (params (InteractingActor :type Actor%20Object%20Reference) (InteractingComponent :type Primitive%20Component%20Object%20Reference))
  (Audio|PlaySound2D "/Game/Audio/Sfx/UI/ShowBody.ShowBody" 1.0 1.0 0.0 0 0)
  (CallFunction|SetTargetHelp (not (Variables|Default|GettargetHelp))))

(event EventBeginPlay
  (|CallParentFunction)
  (Variables|Default|SettargetHelp (Variables|/Game/_Global/BP_SaveGame.BP_SaveGame_C|GettargetHelp (CallFunction|LoadSaveGame "save")))
  (CallFunction|UpdateButtonAppearance))

(fn ConstructionScript
  (|CallParentFunction))

(fn SetTargetHelp
  (params (targetHelp :type Boolean))
  (bind _output_get (Variables|Default|SettargetHelp targetHelp))
  (Default|SetTargetHelp (.AsPlayer (Utilities|Casting|CastToPlayer (Game|Player|GetPlayerPawn 0))) _output_get)
  (bind _output_get_2 (LocalVariables|SetsaveRef (CallFunction|LoadSaveGame "save")))
  (Variables|/Game/_Global/BP_SaveGame.BP_SaveGame_C|SettargetHelp _output_get_2 (Variables|Default|GettargetHelp))
  (SaveGame|SaveGametoSlot (LocalVariables|GetsaveRef) "save")
  (CallFunction|UpdateButtonAppearance))

(fn UpdateButtonAppearance
  (Default|UpdateText (Variables|Default|GetwidgetRef) (select (Variables|Default|GettargetHelp) "ENABLED" "DISABLED") (select (Variables|Default|GettargetHelp) (Utilities|Struct|MakeSlateColor "(R=1.000000,G=0.211561,B=0.781786,A=1.000000)") (Utilities|Struct|MakeSlateColor "(R=0.223958,G=0.000000,B=0.002056,A=1.000000)")))
  (Rendering|SetVisibility (Variables|Default|GetTargetHelpOn) (Variables|Default|GettargetHelp) false)
  (Rendering|SetVisibility (Variables|Default|GetTargetHelpOff) (not (Variables|Default|GettargetHelp)) false))