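; VR menu button that toggles the player's input between controller grips and triggers.
; On BeginPlay it reads the saved preference and updates its widget to a colored GRIPS or TRIGGERS label.
; Each button interaction plays a sound, flips the setting on the Player pawn, saves it, then refreshes its label and the level-select text in BP_Menu.
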(event OnButtonBeginInteraction(VRButton)
  (params (InteractingActor :type Actor%20Object%20Reference) (InteractingComponent :type Primitive%20Component%20Object%20Reference))
  (Audio|PlaySound2D "/Game/Audio/Sfx/Player/Grapple/grapple_hit_Cue.grapple_hit_Cue" 1.0 1.0 0.0 0 0)
  (CallFunction|SetGripUse (not (Variables|Default|GetuseGrips))))

(event EventBeginPlay
  (|CallParentFunction)
  (Variables|Default|SetuseGrips (Variables|/Game/_Global/BP_SaveGame.BP_SaveGame_C|GetuseGripsInsteadOfTriggers (CallFunction|LoadSaveGame "save")))
  (CallFunction|UpdateButtonAppearance))

(fn ConstructionScript
  (|CallParentFunction))

(fn SetGripUse
  (params (useGrips :type Boolean))
  (bind _output_get (Variables|Default|SetuseGrips useGrips))
  (Variables|/Game/Character/Player.Player_C|SetuseGripsInstead (.AsPlayer (Utilities|Casting|CastToPlayer (Game|Player|GetPlayerPawn 0))) _output_get)
  (CallFunction|SaveGame "save")
  (CallFunction|UpdateButtonAppearance)
  (bind _returnvalue (Actor|GetActorOfClass "/Game/UI/Menu/BP_Menu.BP_Menu_C"))
  (Default|UpdateLevelSelectText (Default|GetWMenu _returnvalue)))

(fn UpdateButtonAppearance
  (Default|UpdateText (Variables|Default|GetwidgetRef) (select (Variables|Default|GetuseGrips) "GRIPS" "TRIGGERS") (select (Variables|Default|GetuseGrips) (Utilities|Struct|MakeSlateColor "(R=0.470366,G=0.040252,B=1.000000,A=1.000000)") (Utilities|Struct|MakeSlateColor "(R=1.000000,G=0.653627,B=0.000000,A=1.000000)"))))