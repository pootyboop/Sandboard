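; BP_ZiplinePole is a zipline pole actor that strings a cable to a linked EndPole when play begins.
; BeginPlay calls SetupCable, which, if EndPole is valid, spawns a BP_ZiplineCable at this pole's CableSpawn and attaches it there.
; The cable component's end then attaches to the EndPole's CableSpawn, so the cable exists only at runtime, as the construction script is empty.
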(event EventBeginPlay
  (CallFunction|SetupCable))

(fn ConstructionScript)

(fn SetupCable
  (bind _cablespawn (Variables|Default|GetcableSpawn))
  (bind _returnvalue (Transformation|GetWorldTransform _cablespawn))
  (Variables|Default|GetendPole
    (:then
      (bind _returnvalue_2 (Game|SpawnActorfromClass "/Game/MeshesAndWorldStuff/WoodAndDecoration/Zipline/BP_ZiplineCable.BP_ZiplineCable_C" (Math|Transform|MakeTransform (.location _returnvalue) (.rotation _returnvalue) "1,1,1") "Undefined" 0 0))
      (Transformation|AttachComponentToComponent _returnvalue_2 (Variables|Default|GetcableSpawn) "None" "KeepWorld" "KeepWorld" "KeepWorld" true)
      (Class|CableComponent|SetAttachEndtoComponent (Variables|/Script/CableComponent.CableActor|GetCableComponent _returnvalue_2) (Variables|BP_ZiplinePole_C|GetcableSpawn (Variables|Default|GetendPole)) "None"))
    (:else)))