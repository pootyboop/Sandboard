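; BP_TargetSpinner is a level actor that rotates a set of four BP_Target child actors.
; Tick adds local pitch rotation to the Spinner component, scaled by SpinSpeed and delta time.
; The construction script gathers the child targets into a unique TiedActors list, then copies that list to each target so they all reference the whole group.
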(event EventBeginPlay)

(event Collision|EventActorBeginOverlap
  (params (OtherActor :type Actor%20Object%20Reference)))

(event EventTick
  (params (DeltaSeconds :type Float%20%28single-precision%29))
  (Transformation|AddLocalRotation (Variables|Default|GetSpinner) (Math|Rotator|MakeRotator 0.0 (* DeltaSeconds (Variables|Default|GetspinSpeed)) 0.0) false false))

(fn ConstructionScript
  (bind _target1 (Variables|Default|GetTarget1))
  (bind _target2 (Variables|Default|GetTarget2))
  (bind _target3 (Variables|Default|GetTarget3))
  (bind _target (Variables|Default|GetTarget))
  (bind _array (Utilities|Array|MakeArray _target1 _target2 _target3 _target))
  (for _array_element _array
    (Utilities|Array|AddUnique (Variables|Default|GettiedActors) (.AsBP%20Target (Utilities|Casting|CastToBP_Target (Variables|/Script/Engine.ChildActorComponent|GetChildActor _array_element)))))
  (for _array_element_2 _array
    (Variables|/Game/MeshesAndWorldStuff/LevelFunction/BP_Target.BP_Target_C|SettiedActors (.AsBP%20Target (Utilities|Casting|CastToBP_Target (Variables|/Script/Engine.ChildActorComponent|GetChildActor _array_element_2))) (Variables|Default|GettiedActors))))