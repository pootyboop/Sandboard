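; Rail actor that carries the player along a spline from a start sphere to the end, like a rail ride.
; The construction script builds two mirrored rows of spline meshes, offset either side of the spline.
; On overlap, the player enters rail movement and attaches to MovingPoint, which a fast looping timer advances by MoveSpeed.
; At the end, the player detaches and the rail resets for reuse.
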(event OnComponentBeginOverlap(StartSphere)
  (params (OverlappedComponent :type Primitive%20Component%20Object%20Reference) (OtherActor :type Actor%20Object%20Reference) (OtherComp :type Primitive%20Component%20Object%20Reference) (OtherBodyIndex :type Integer) (bFromSweep :type Boolean) (SweepResult :type Hit%20Result%20Structure%20%28by%20ref%29))
  (bind _asplayer (Utilities|Casting|CastToPlayer OtherActor))
  (Utilities|FlowControl|DoOnce false
    (:Completed
      (Variables|Default|Setplayer _asplayer)
      (CallFunction|StartMoving))))

(event Custom|StartMoving
  (Default|SetRailMovement (Variables|Default|Getplayer) true)
  (Transformation|AttachComponentToComponent (Variables|Default|Getplayer) (Variables|Default|GetMovingPoint) "None" "KeepWorld" "KeepWorld" "KeepWorld" true)
  (Variables|Default|SetprevRot (Transformation|GetActorRotation (Variables|Default|Getplayer)))
  (bind _returnvalue (Utilities|Time|SetTimerbyEvent (delegate Custom|Move) 0.005 true))
  (Variables|Default|SettimerHandle _returnvalue))

(event Custom|EndMoving
  (Utilities|Time|ClearandInvalidateTimerbyHandle (Variables|Default|GettimerHandle))
  (Transformation|DetachFromActor (Variables|Default|Getplayer) "KeepWorld" "KeepWorld" "KeepWorld")
  (Default|SetRailMovement (Variables|Default|Getplayer) false)
  (Variables|Default|Setdistance 0.0)
  (Transformation|SetRelativeLocationAndRotation (Variables|Default|GetMovingPoint) "0, 0, 0" "0, 0, 0" false false)
  (CallFunction|ResetRailUsable))

(event Custom|Move
  (CallFunction|MoveAlongSpline))

(event Custom|ResetRailUsable
  (Utilities|FlowControl|DoOnce false) ; enters at Reset
)

(event EventBeginPlay
  (Variables|Default|Setlength (Spline|GetSplineLength (Variables|Default|GetSpline))))

(event Collision|EventActorBeginOverlap
  (params (OtherActor :type Actor%20Object%20Reference)))

(event EventTick
  (params (DeltaSeconds :type Float%20%28single-precision%29)))

(fn ConstructionScript
  (CallFunction|SetupRail))

(fn SetupRail
  (for _index (range 0 (- (Spline|GetNumberOfSplinePoints (Variables|Default|GetSpline)) 2))
    (CallFunction|AddSegment _index)))

(fn AddSegment
  (params (index :type Integer))
  (bind _railoffset (Variables|Default|GetrailOffset))
  (CallFunction|AddRailMesh index (Variables|Default|GetrailOffset))
  (CallFunction|AddRailMesh index (Math|Transform|MakeTransform (Math|Vector|MakeVector (.x (.location _railoffset)) (* -1 (.y (.location _railoffset))) (.z (.location _railoffset))) (.rotation _railoffset) (.scale _railoffset))))

(fn AddRailMesh
  (params (index :type Integer) (offset :type Transform))
  (bind _spline (Variables|Default|GetSpline))
  (bind _spline_2 (Variables|Default|GetSpline))
  (bind _returnvalue (+ index 1))
  (bind _returnvalue_2 (AddComponent|AddSplineMeshComponent true))
  (SplineMesh|SetForwardAxis _returnvalue_2 "X" true)
  (SplineMesh|SetStartandEnd _returnvalue_2 (CallFunction|TranslatePositiontoRailOffset (Spline|GetLocationatSplinePoint _spline_2 index "World") offset index) (Spline|GetTangentatSplinePoint _spline_2 index "World") (CallFunction|TranslatePositiontoRailOffset (Spline|GetLocationatSplinePoint _spline _returnvalue "World") offset _returnvalue) (Spline|GetTangentatSplinePoint _spline _returnvalue "World") true :!class /Script/Engine.SplineMeshComponent))

(fn TranslatePositiontoRailOffset
  (params (worldPosition :type Vector) (localTransform :type Transform) (splineIndex :type Integer))
  (return (+ (Math|Vector|RotateVector (.Location (Math|Transform|BreakTransform localTransform)) (Spline|GetRotationatSplinePoint (Variables|Default|GetSpline) splineIndex "World")) worldPosition)))

(fn MoveAlongSpline
  (bind _spline (Variables|Default|GetSpline))
  (bind _output_get (Variables|Default|Setdistance (+ (Variables|Default|GetmoveSpeed) (Variables|Default|Getdistance))))
  (if (< _output_get (Variables|Default|Getlength))
    (Transformation|SetRelativeLocationAndRotation (Variables|Default|GetMovingPoint) (Spline|GetLocationatDistanceAlongSpline _spline (Variables|Default|Getdistance) "Local") (Spline|GetRotationatDistanceAlongSpline _spline (Variables|Default|Getdistance) "Local") false false)
    (Transformation|SetActorRelativeLocation (Variables|Default|Getplayer))
    (Transformation|SetActorRelativeRotation (Variables|Default|Getplayer))
    (else
      (CallFunction|EndMoving))))