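; BP_Target is a one-shot level target that triggers linked actors when its mesh is hit.
; Its grapple point stays only if the saved TargetHelp option is on, and is destroyed once the target is used.
; A hit swaps a material, plays a sound and calls TriggerInteraction on every TiedActor.
; Activation through TriggerInteraction also disables the target but skips sound and propagation, so triggers do not chain.
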(event OnComponentHit(target)
  (params (HitComponent :type Primitive%20Component%20Object%20Reference) (OtherActor :type Actor%20Object%20Reference) (OtherComp :type Primitive%20Component%20Object%20Reference) (NormalImpulse :type Vector :default "0, 0, 0") (Hit :type Hit%20Result%20Structure%20%28by%20ref%29))
  (CallFunction|OnHit false))

(event Custom|OnHit
  (params (fromInteraction :type Boolean))
  (Utilities|FlowControl|DoOnce false
    (:Completed
      (Rendering|Material|SetMaterial (Variables|Default|Gettarget) 1 "/Engine/MapTemplates/Sky/M_BlackBackground.M_BlackBackground")
      (bind _grapple_point (Variables|Default|GetGrapple%20Point)
        (:then
          (Components|DestroyComponent _grapple_point))
        (:else
          _))
      (if (not fromInteraction)
        (Audio|PlaySound2D "/Game/Audio/Sfx/World/target_hit_Cue.target_hit_Cue" 1.0 1.0 0.0 0 0)
        (for _array_element (Variables|Default|GettiedActors)
          (Default|TriggerInteraction _array_element))))))

(event EventBeginPlay
  (if (not (Variables|/Game/_Global/BP_SaveGame.BP_SaveGame_C|GettargetHelp (CallFunction|LoadSaveGame "save")))
    (Components|DestroyComponent (Variables|Default|GetGrapple%20Point))))

(event EventTriggerInteraction
  (CallFunction|OnHit true))

(fn ConstructionScript)