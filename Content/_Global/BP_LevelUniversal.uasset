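; Universal level Blueprint that sets up shared per-level behavior: background music, fullscreen and a fall-death check.
; BeginPlay plays the music from the Levels data table row matching the current level name, then runs the fullscreen console command.
; StartFallCheck starts a looping timer that compares the player board's world Y, not Z, to FallDeathZ and only prints a death message.
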(event Custom|StartFallCheck
  (if (!= (Variables|Default|GetfallDeathZ) 0.0)
    (bind _asplayer (Utilities|Casting|CastToPlayer (Game|Player|GetPlayerPawn 0)))
    (Variables|Default|Setplayer _asplayer)
    (Utilities|Time|SetTimerbyEvent (delegate Custom|FallCheck) 2.0 true)))

(event Custom|FallCheck
  (if (< (.y (Transformation|GetWorldLocation (Variables|/Game/Character/Player.Player_C|GetBP_Sandboard (Variables|Default|Getplayer)))) (Variables|Default|GetfallDeathZ))
    (Development|PrintString "PLAYER DEAD!!!! -from BP_LevelUniversal for going under fallDeathZ")))

(event EventBeginPlay
  (Utilities|FlowControl|Sequence
    (:then_0
      (CallFunction|StartMusic))
    (:then_1
      (Utilities|FlowControl|Delay 0.1)
      (Development|ExecuteConsoleCommand "fullscreen" 0))))

(fn ConstructionScript)

(fn Fullscreen)

(fn StartMusic
  (bind _outrownames (DataTable|GetDataTableRowNames "/Game/UI/Levels/Levels.Levels"))
  (for _array_element _outrownames
    (bind _returnvalue (Utilities|GetDataTableRow "/Game/UI/Levels/Levels.Levels" _array_element)
      (:then
        (bind _returnvalue_2 (Game|GetCurrentLevelName true))
        (if (Utilities|Name|Equal(Name) (Utilities|String|StringToName _returnvalue_2) (CallFunction|DatatableNametoLevelName (.Name (Utilities|Struct|BreaksLevel _returnvalue))))
          (Utilities|IsValid (.Music (Utilities|Struct|BreaksLevel _returnvalue))
            (:Is%20Valid
              (CallFunction|PlayBGM (.Music (Utilities|Struct|BreaksLevel _returnvalue))))))))))