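; BP_FunctionLibrary is a global function library of shared helpers for time display, level checks, game state access and music playback.
; ToSeconds turns a seconds count into colon-separated text by counting off minutes in a loop and zero-padding the remaining seconds.
; InLevel compares a name against the current level.
; GetGameState returns the state cast to GS_Global, which PlayBGM reads for MusicVolume when playing a 2D sound.
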(fn ToSeconds
  (params (Time :type Float%20%28single-precision%29))
  (LocalVariables|SettimeLeft Time)
  (while (>= (LocalVariables|GettimeLeft) 6e+01)
    (LocalVariables|SettimeLeft (- (LocalVariables|GettimeLeft) 6e+01))
    (Math|Integer|IncrementInt (LocalVariables|GetMinutes)))
  (return (Utilities|Text|ToText(String) (Utilities|String|Replace (Utilities|String|Append (Utilities|String|ToString(Integer) (LocalVariables|GetMinutes)) "." (Utilities|String|SelectString "0" "" (< (LocalVariables|GettimeLeft) 1e+01)) (Utilities|String|ToString(Text) (Utilities|Text|ToText(Float) (LocalVariables|GettimeLeft) "HalfToEven"))) "." ":"))))

(fn InLevel
  (params (levelName :type String))
  (bind _returnvalue (Game|GetCurrentLevelName 0))
  (return (Utilities|Enum|Equal(Enum) _returnvalue levelName)))

(fn GetGameState
  (bind _asgs_global (Utilities|Casting|CastToGS_Global (Game|GetGameState)))
  (return _asgs_global))

(fn PlayBGM
  (params (Music :type Sound%20Base%20Object%20Reference))
  (Audio|PlaySound2D 0 Music (Variables|/Game/_Global/GS_Global.GS_Global_C|GetmusicVolume (CallFunction|GetGameState)) 1.0 0.0 0 0 false))